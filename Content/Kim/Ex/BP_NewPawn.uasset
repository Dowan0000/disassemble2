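; Experimental camera pawn with spring-arm zoom, yaw-relative forward movement and data-table-driven camera moves.
; ActorChangeTransform looks up a row and runs a timeline that eases the collision component toward its CameraTransform and the arm length to 50, re-reading current values each update.
; BeginPlay collects numbered Transform-tagged ArrowActors into an array, only printed here.
; The Rotate axis does no rotation, just a one-time debug print of row "1-1".
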(event `InputAction|ZoomIn2`
  (params (Key :type "Key Structure"))
  (bind _springarm (`self.SpringArm`))
  (:`Pressed`
    (set `SpringArmComponent.TargetArmLength` (- (`SpringArmComponent.TargetArmLength` _springarm) (* 1.0 10.0)) _springarm)))

(event `InputAction|ZoomOut2`
  (params (Key :type "Key Structure"))
  (bind _springarm (`self.SpringArm`))
  (:`Pressed`
    (set `SpringArmComponent.TargetArmLength` (+ (* 1.0 10.0) (`SpringArmComponent.TargetArmLength` _springarm)) _springarm)))

(event `InputAxis|Rotate`
  (params (AxisValue :type "Float (single-precision)"))
  (`/Engine/EditorBlueprintResources/StandardMacros.DoOnce` false
    (:`Completed`
      (bind _returnvalue (`|GetDataTableRow` "/Game/ThirdPerson/Blueprints/Ex/NewDataTable.NewDataTable" "1-1")
        (:`then`
          (bind _output_get (set `self.Struct` _returnvalue))
          (bind (_markedfirstframe _markedlastframe _cameratransform _textstruct) (break `/Game/ThirdPerson/Blueprints/Ex/NewUserDefinedStruct` _output_get))
          (`KismetSystemLibrary.PrintString` _markedfirstframe true true (struct :`R` 0.782487 :`G` 1.0 :`A` 1.0) 10.0)
          (`KismetSystemLibrary.PrintString` _markedlastframe true true (struct :`R` 0.782487 :`G` 1.0 :`A` 1.0) 10.0)
          (`KismetSystemLibrary.PrintString` (`KismetStringLibrary.Conv_TransformToString` _cameratransform) true true (struct :`R` 0.782487 :`G` 1.0 :`A` 1.0) 10.0)
          (bind (_index _text1) (break `/Game/ThirdPerson/Blueprints/Ex/NewUserDefinedStruct1` _textstruct))
          (`KismetSystemLibrary.PrintString` _index true true (struct :`R` 0.782487 :`G` 1.0 :`A` 1.0) 10.0)
          (`KismetSystemLibrary.PrintString` _text1 true true (struct :`R` 0.782487 :`G` 1.0 :`A` 1.0) 10.0))))))

(event `InputAxis|Move`
  (params (AxisValue :type "Float (single-precision)"))
  (bind (_returnvalue_roll _returnvalue_pitch _returnvalue_yaw) (`KismetMathLibrary.BreakRotator` (`self.GetControlRotation`)))
  (`self.AddMovementInput` (`KismetMathLibrary.GetForwardVector` (`KismetMathLibrary.MakeRotator` 0.0 0.0 _returnvalue_yaw)) AxisValue))

(event `self.ReceiveBeginPlay`
  (bind _transformarray (`self.TransformArray`))
  (for _index (range 1 6)
    (bind _outactors (`GameplayStatics.GetAllActorsOfClassWithTag` "/Game/ThirdPerson/Blueprints/Ex/ArrowActor.ArrowActor_C" (`KismetStringLibrary.Conv_StringToName` (`KismetStringLibrary.Concat_StrStr` "Transform" (`KismetStringLibrary.Conv_IntToString` _index)))))
    (for _array_element _outactors
      (bind _asarrow_actor (cast `/Game/ThirdPerson/Blueprints/Ex/ArrowActor` _array_element))
      (`KismetSystemLibrary.PrintString` (`KismetSystemLibrary.GetDisplayName` _asarrow_actor))
      (`KismetArrayLibrary.Array_Add` _transformarray _asarrow_actor))
    (for _array_element_2 _transformarray
      (`KismetSystemLibrary.PrintString` (`KismetSystemLibrary.GetDisplayName` _array_element_2) true true (struct :`R` 1.0 :`G` 0.834869 :`A` 1.0) 10.0))))

(event `ActorChangeTransform`
  (params (RowName :type String))
  (bind _returnvalue (`|GetDataTableRow` "/Game/ThirdPerson/Blueprints/Ex/NewDataTable.NewDataTable" (`KismetStringLibrary.Conv_StringToName` RowName))
    (:`then`
      (bind (_direction `_새_트랙_0`) (`Timeline|타임라인_0` :!via `PlayFromStart`)
        (:`Update`
          (`SceneComponent.K2_SetWorldTransform` (`self.CollisionComponent`) (`|EaseFunction` "CircularIn" `_새_트랙_0` (`SceneComponent.K2_GetComponentToWorld` (`self.CollisionComponent`)) (`.CameraTransform_11_4A8F696E41990B5084263E9D811EE821` (break `/Game/ThirdPerson/Blueprints/Ex/NewUserDefinedStruct` _returnvalue))) false false)
          (set `SpringArmComponent.TargetArmLength` (`|EaseFunction` "CircularIn" `_새_트랙_0` (`SpringArmComponent.TargetArmLength` (`self.SpringArm`)) 50.0) (`self.SpringArm`)))
        (:`Finished`
          (`KismetSystemLibrary.PrintString` "ChangeFinished" true true (struct :`R` 0.254749 :`G` 1.0 :`A` 1.0) 10.0))))))

(fn `UserConstructionScript`)